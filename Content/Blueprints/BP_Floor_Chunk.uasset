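; BP_Floor_Chunk is one row of floor in a chicken-crossing game, holding left, center and right floors, landing nodes and props.
; Helper functions compute the three floor transforms, spawn landing nodes along X with a water flag, and randomly spawn coins at the running node position.
; A BeginPlay timer calls a check that destroys the chunk and its tracked actors if its Y offset from the chicken reaches a limit.
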(event EventBeginPlay
  (Utilities|Time|SetTimerbyFunctionName 0 "CheckIfDestroyFloorChunk" 1.0))

(fn ConstructionScript)

(fn CalcFloorTransform
  (bind _positiony (Variables|Default|GetPositionY))
  (return (Math|Transform|MakeTransform (Math|Vector|MakeVector -1.8e+03 _positiony 0.0)) (Math|Transform|MakeTransform (Math|Vector|MakeVector 0.0 _positiony 0.0)) (Math|Transform|MakeTransform (Math|Vector|MakeVector 1.8e+03 _positiony 0.0)) _positiony))

(fn DestroyMeshesLandingNodesandProps
  (for _array_element (Variables|Default|GetLandingNodes)
    (Actor|DestroyActor _array_element))
  (Actor|DestroyActor (Variables|Default|GetLeftFloor))
  (Actor|DestroyActor (Variables|Default|GetRightFloor))
  (Actor|DestroyActor (Variables|Default|GetCenterFloor))
  (for _array_element_2 (Variables|Default|GetProps)
    (Actor|DestroyActor _array_element_2)))

(fn CheckifDestroyFloorChunk
  (bind _chickenref (Variables|Default|GetChickenREF))
  (Utilities|IsValid _chickenref
    (:Is%20Valid
      (if (>= (.y (Transformation|GetActorLocation)) (+ (.y (Transformation|GetActorLocation _chickenref)) (Variables|Default|GetMaxDistanceBackwardsFromChicken)))
        (CallFunction|DestroyMeshesLandingNodesandProps)
        (Actor|DestroyActor)))))

(fn ConstructLandingNode(FloorChunk)
  (params (IsWater :type Boolean))
  (bind _returnvalue (Game|SpawnActorfromClass "/Game/Blueprints/BP_LandingNode.BP_LandingNode_C" (Math|Transform|MakeTransform (Math|Vector|MakeVector (Variables|Default|GetCurrentXPosFromLandingNode) (.y (Transformation|GetActorLocation)) (Variables|Default|GetCurrentZPosFromLandingNode))) "Undefined" 0 IsWater 0))
  (Variables|Default|SetCurrentXPosFromLandingNode (+ (Variables|Default|GetCurrentXPosFromLandingNode) 2e+02))
  (Utilities|Array|Add (Variables|Default|GetLandingNodes) _returnvalue))

(fn AttemptingCoinCreation
  (if (== (Math|Random|RandomInteger 9) 0)
    (Game|SpawnActorfromClass "/Game/Blueprints/BP_Coin.BP_Coin_C" (Math|Transform|MakeTransform (Math|Vector|MakeVector (Variables|Default|GetCurrentXPosFromLandingNode) (.y (Transformation|GetActorLocation)) (Variables|Default|GetCurrentZPosFromLandingNode))) "Undefined" 0 0)))