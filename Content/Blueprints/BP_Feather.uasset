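; BP_Feather is an actor that tumbles as it falls through the world, presumably as a feather effect.
; BeginPlay picks a random starting rotation and caches the actor's location.
; Each Tick advances all three rotation axes and lowers Z at constant, frame-rate-independent rates, setting the transform directly without sweep or physics, and nothing stops the fall.
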(event EventBeginPlay
  (Variables|Default|SetRotation (Math|Random|RandomRotator false))
  (Variables|Default|SetLocation (Transformation|GetActorLocation)))

(event EventTick
  (params (DeltaSeconds :type Float%20%28single-precision%29))
  (bind _returnvalue (* DeltaSeconds 1e+02))
  (bind _output_get (Variables|Default|SetRotation (Math|Rotator|MakeRotator (+ (.roll (Variables|Default|GetRotation)) _returnvalue) (+ (.pitch (Variables|Default|GetRotation)) _returnvalue) (+ (.yaw (Variables|Default|GetRotation)) _returnvalue))))
  (Transformation|SetActorRotation _output_get)
  (bind _output_get_2 (Variables|Default|SetLocation (Math|Vector|MakeVector (.x (Variables|Default|GetLocation)) (.y (Variables|Default|GetLocation)) (+ (.z (Variables|Default|GetLocation)) (* DeltaSeconds -1e+02)))))
  (Transformation|SetActorLocation _output_get_2 false false))

(fn ConstructionScript)