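; BP_Train is a train actor that travels in a straight line along the world X axis and removes itself after a set time.
; On BeginPlay, MoveLeft turns it 180 degrees to face the opposite direction.
; Each Tick offsets it by MoveSpeed scaled by delta time, toward negative X when MoveLeft is set, then counts LifeTime down and destroys the actor at zero.
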(event EventBeginPlay
  ;[1 1 1] If Move Oposite, Rotate to 180
  (if (Variables|Default|GetMoveLeft)
    (Transformation|SetActorRotation "0,180.000000, 0")))

(event EventTick
  (params (DeltaSeconds :type Float%20%28single-precision%29))
  ;[1 1 1] Move Train
  (if (Variables|Default|GetMoveLeft)
    (Transformation|AddActorWorldOffset (Math|Vector|MakeVector (* (* (Variables|Default|GetMoveSpeed) DeltaSeconds) -1.0) 0.0 0.0))
    (else
      (Transformation|AddActorWorldOffset (Math|Vector|MakeVector (* DeltaSeconds (Variables|Default|GetMoveSpeed)) 0.0 0.0))))
  ;[1 1 1] Handle Train LifeTime
  (Variables|Default|SetLifeTime (- (Variables|Default|GetLifeTime) DeltaSeconds))
  (if (<= (Variables|Default|GetLifeTime) 0.0)
    (Actor|DestroyActor)))

(fn ConstructionScript)