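; Water lane floor chunk for a Frogger-style crossing, spawning three floor sections, landing nodes and optional lily pads or drifting logs.
; Lily pads spawn from clear-column positions and are destroyed with the chunk.
; Logs pre-fill the lane at BeginPlay, then Tick spawns more off to one side on a randomized timer.
; Each log's random length and the lane's shared random speed bonus set the delay before the next.
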(event EventBeginPlay
  (|CallParentFunction)
  (bind (_transformleft _transformmid _transofrmright) (CallFunction|CalcFloorTransform))
  (Utilities|FlowControl|Sequence
    (:then_0
      (bind _returnvalue (Game|SpawnActorfromClass "/Game/Blueprints/BP_Floor.BP_Floor_C" _transformleft "Undefined" 0 2 false self 0))
      (Variables|Default|SetLeftFloor _returnvalue))
    (:then_1
      (bind _returnvalue_2 (Game|SpawnActorfromClass "/Game/Blueprints/BP_Floor.BP_Floor_C" _transformmid "Undefined" 0 2 true self 0))
      (Variables|Default|SetCenterFloor _returnvalue_2))
    (:then_2
      (bind _returnvalue_3 (Game|SpawnActorfromClass "/Game/Blueprints/BP_Floor.BP_Floor_C" _transofrmright "Undefined" 0 2 false self 0))
      (Variables|Default|SetRightFloor _returnvalue_3))
    (:then_3
      (CallFunction|ConstructLandingNodes)
      (if (Variables|Default|GetCreateLogs)
        (CallFunction|ConstructInitialLogs)))))

(event EventTick
  (params (DeltaSeconds :type Float%20%28single-precision%29))
  (|CallParentFunction DeltaSeconds)
  (if (Variables|Default|GetCreateLogs)
    (CallFunction|ConstructLogAttempt DeltaSeconds)))

(event EventDestroyed
  (for _array_element (Variables|Default|GetLilyPads)
    (Actor|DestroyActor _array_element)))

(fn ConstructionScript
  (|CallParentFunction)
  (if (Variables|Default|GetCreateLogs)
    (Variables|Default|SetMaxCreateLogTime (Math|Random|RandomFloatinRange 0.0 1.0))
    (CallFunction|AddExtraLogSpeedRandom)))

(fn ConstructLilyPad
  (params (CurrentX :type Float%20%28single-precision%29))
  (bind _returnvalue (Transformation|GetActorLocation))
  (if (== CurrentX -1.0)
    (bind _returnvalue_2 (Game|SpawnActorfromClass "/Game/Blueprints/BP_LilyPad.BP_LilyPad_C" (Math|Transform|MakeTransform (Math|Vector|MakeVector CurrentX (.y _returnvalue) (- (.z _returnvalue) 3e+01)) "0, 0, 0" "1,1,1") "Undefined" 0 0))
    (Utilities|Array|Add (Variables|Default|GetLilyPads) _returnvalue_2)))

(fn ConstructLilyPads(Multiple)
  (bind _currentclearcolumnposx3 (Variables|Default|GetCurrentClearColumnPosX3))
  ;[1 1 1] Try Construct First LilyPad
  (if (>= (Variables|Default|GetNumberOfLilyPadsToCreate) 1)
    (CallFunction|ConstructLilyPad (Variables|Default|GetCurrentClearColumnPosX1))
    ;[1 1 1] Try Construct Second LiliPad
    (if (>= (Variables|Default|GetNumberOfLilyPadsToCreate) 2)
      (if (!= (Variables|Default|GetCurrentClearColumnPosX1) (Variables|Default|GetCurrentClearColumnPosX2))
        (CallFunction|ConstructLilyPad (Variables|Default|GetCurrentClearColumnPosX2))
        ;[1 1 1] Try Construct Third LilyPad
        (if (>= (Variables|Default|GetNumberOfLilyPadsToCreate) 3)
          (if (or (!= (Variables|Default|GetCurrentClearColumnPosX2) _currentclearcolumnposx3) (!= _currentclearcolumnposx3 (Variables|Default|GetCurrentClearColumnPosX1)))
            (CallFunction|ConstructLilyPad (Variables|Default|GetCurrentClearColumnPosX3))))))))

(fn ConstructLandingNodes
  (Variables|Default|SetCurrentZPosFromLandingNode -6e+01)
  (for _index (range 0 8)
    (CallFunction|ConstructLandingNode(FloorChunk) true))
  (if (Variables|Default|GetCreateLilyPads)
    (CallFunction|ConstructLilyPads(Multiple))))

(fn ConstructLog
  (params (LocationX :type Float%20%28single-precision%29))
  (bind _returnvalue (Transformation|GetActorLocation))
  (bind _returnvalue_2 (Game|SpawnActorfromClass "/Game/Blueprints/BP_Log.BP_Log_C" (Math|Transform|MakeTransform (Math|Vector|MakeVector LocationX (.y _returnvalue) (.z _returnvalue))) "Undefined" 0 (Math|Random|RandomIntegerinRange 1 3) (not (Variables|Default|GetCreateLogsLeft)) (Variables|Default|GetExtraLogSpeedCenter) 0))
  (bind _output_get (Variables|Default|SetCurrentLogCreated _returnvalue_2))
  (return _output_get))

(fn CalcLogCreationOffsetNext
  (Utilities|IsValid (Variables|Default|GetCurrentLogCreated)
    (:Is%20Valid
      (switch int (Variables|/Game/Blueprints/BP_Log.BP_Log_C|GetLength (Variables|Default|GetCurrentLogCreated))
        (:1
          (return (Math|Random|RandomFloatinRange 4e+02 5e+02)))
        (:2
          (return (Math|Random|RandomFloatinRange 6e+02 7e+02)))
        (:3
          (return (Math|Random|RandomFloatinRange 8e+02 9e+02)))))
    (:Is%20Not%20Valid
      (return (Math|Random|RandomFloatinRange 0.0 1e+02)))))

(fn ConstructInitialLogs
  (if (Variables|Default|GetCreateLogsLeft)
    (LocalVariables|SetLogCreateXPos -9e+02)
    (while (< (LocalVariables|GetLogCreateXPos) 9e+02)
      (bind _randxpos (CallFunction|CalcLogCreationOffsetNext))
      (bind _output_get (LocalVariables|SetLogCreateXPos (+ _randxpos (LocalVariables|GetLogCreateXPos))))
      (CallFunction|ConstructLog _output_get))
    (else
      (LocalVariables|SetLogCreateXPos 9e+02)
      (while (> (LocalVariables|GetLogCreateXPos) -9e+02)
        (bind _randxpos_2 (CallFunction|CalcLogCreationOffsetNext))
        (bind _output_get_2 (LocalVariables|SetLogCreateXPos (- (LocalVariables|GetLogCreateXPos) _randxpos_2)))
        (CallFunction|ConstructLog _output_get_2)))))

(fn AddExtraLogSpeedRandom
  (Variables|Default|SetExtraLogSpeedCenter (Math|Random|RandomFloatinRange 0.0 2e+02)))

(fn ConstructLogAttempt
  (params (DeltaSeconds :type Float%20%28single-precision%29))
  (bind _output_get (Variables|Default|SetCurrentCreateLogTime (+ DeltaSeconds (Variables|Default|GetCurrentCreateLogTime))))
  (if (>= _output_get (Variables|Default|GetMaxCreateLogTime))
    (if (Variables|Default|GetCreateLogsLeft)
      (CallFunction|ConstructLog -2.8e+03)
      (else
        (CallFunction|ConstructLog 2.8e+03)))
    (Variables|Default|SetCurrentCreateLogTime 0.0)
    (switch int (Variables|/Game/Blueprints/BP_Log.BP_Log_C|GetLength (Variables|Default|GetCurrentLogCreated))
      (:1
        (Variables|Default|SetMaxCreateLogTime (- (Math|Random|RandomFloatinRange 1.25 1.5) (/ (Variables|Default|GetExtraLogSpeedCenter) 4e+02))))
      (:2
        (Variables|Default|SetMaxCreateLogTime (- (Math|Random|RandomFloatinRange 1.5 1.75) (/ (Variables|Default|GetExtraLogSpeedCenter) 4e+02))))
      (:3
        (Variables|Default|SetMaxCreateLogTime (- (Math|Random|RandomFloatinRange 2.0 2.25) (/ (Variables|Default|GetExtraLogSpeedCenter) 4e+02)))))))