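; Chicken actor for a Crossy Road-style hopper, with helpers for jumping between landing nodes, lily pads and logs.
; A downward trace picks the landing target and flags water falls, while log jumps use an X offset.
; Helpers compute crouch scale, linear movement and a parabolic hop height, or move the chicken along with cars and logs.
; The event graph and jump-sound function are empty, and nothing here drives the movement helpers.
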(event EventBeginPlay)

(event Collision|EventActorBeginOverlap
  (params (OtherActor :type Actor%20Object%20Reference)))

(event EventTick
  (params (DeltaSeconds :type Float%20%28single-precision%29)))

(fn ConstructionScript)

(fn ProcessChickenSquishedFwd
  (params (DeltaSeconds :type Float%20%28single-precision%29))
  (bind _curcar (Variables|Default|GetCurCar))
  (bind _speed (Variables|/Game/Blueprints/BP_Vehicle.BP_Vehicle_C|GetSpeed _curcar))
  (bind _returnvalue (* DeltaSeconds _speed))
  (Utilities|IsValid _curcar
    (:Is%20Valid
      (if (Variables|/Game/Blueprints/BP_Vehicle.BP_Vehicle_C|GetMoveLeft _curcar)
        (Variables|Default|SetCurCarVelX (* _returnvalue -1.0))
        (else
          (Variables|Default|SetCurCarVelX _returnvalue)))
      (Transformation|AddActorWorldOffset (Math|Vector|MakeVector (Variables|Default|GetCurCarVelX) 0.0 0.0)))))

(fn ProcessChickenCarriedOffbyLog
  (params (DeltaSeconds :type Float%20%28single-precision%29))
  (bind _curlog (Variables|Default|GetCurLog))
  (bind _currentspeed (Variables|/Game/Blueprints/BP_Log.BP_Log_C|GetCurrentSpeed _curlog))
  (bind _returnvalue (* DeltaSeconds _currentspeed))
  (Utilities|IsValid _curlog
    (:Is%20Valid
      (if (Variables|/Game/Blueprints/BP_Log.BP_Log_C|GetMoveLeft _curlog)
        (Variables|Default|SetCurCarVelX _returnvalue)
        (else
          (Variables|Default|SetCurCarVelX _returnvalue)))
      (Transformation|AddActorWorldOffset (Math|Vector|MakeVector (Variables|Default|GetCurCarVelX) 0.0 0.0)))))

(fn CrouchAnim
  (params (DeltaSeconds :type Float%20%28single-precision%29))
  (if (< (Variables|Default|GetCrouchAmount) 1.0)
    (Variables|Default|SetCrouchAmount (+ (* DeltaSeconds 8.0) (Variables|Default|GetCrouchAmount)))
    (Variables|Default|SetCrouchScale (Math|Float|Lerp 1.0 (LocalVariables|GetCrouchFinalAmount) (Variables|Default|GetCrouchAmount)))
    (else
      (Variables|Default|SetCrouchScale (LocalVariables|GetCrouchFinalAmount)))))

(fn CalcNewNodePos
  (params (NodeObj :type Actor%20Object%20Reference))
  (bind _returnvalue (Transformation|GetActorLocation))
  (bind _curdir (Variables|Default|GetCurDir))
  (bind _returnvalue_2 (Transformation|GetActorLocation NodeObj))
  (bind (_x _y _z) (Math|Vector|BreakVector _returnvalue_2))
  (if (Variables|Default|GetIsOnLilyPad)
    (bind _output_get (Variables|Default|SetCurLandingNodePos _returnvalue_2 :!label _label))
    (Variables|Default|SetDistToLandingNode (Math|Vector|Distance(Vector) _output_get _returnvalue))
    (else
      (bind _asbp_landing_node (Utilities|Casting|CastToBP_LandingNode NodeObj))
      (if (Variables|/Game/Blueprints/BP_LandingNode.BP_LandingNode_C|GetIs%20Water _asbp_landing_node)
        (if (or (== _curdir 3) (== _curdir 2))
          (bind _output_get_2 (Variables|Default|SetCurLandingNodePos (Math|Vector|MakeVector (.X (Math|Vector|BreakVector _returnvalue)) _y _z)))
          (Variables|Default|SetDistToLandingNode (Math|Vector|Distance(Vector) _output_get_2 (Transformation|GetActorLocation)))
          (else
            (goto _label)))
        (else
          (goto _label))))))

(fn PlayJumpingSounds)

(fn TraceforLandingNode
  (params (RayStart :type Vector) (RayEnd :type Vector))
  (bind _outhits (Collision|MultiLineTraceByChannel RayStart RayEnd "TraceTypeQuery1" false 0 "ForDuration" true "(R=1.000000,G=0.000000,B=0.000000,A=1.000000)" "(R=0.000000,G=1.000000,B=0.000000,A=1.000000)" 16.0))
  (bind _array_element (Utilities|Array|ForEachLoopwithBreak _outhits :!label _label)
    (:LoopBody
      (bind _asbp_landing_node (Utilities|Casting|CastToBP_LandingNode (.HitActor (Collision|BreakHitResult _array_element)))
        (:then
          (Variables|Default|SetCurLandingNode _asbp_landing_node)
          (Variables|Default|SetIsOnLog false)
          (Variables|Default|SetFoundLandingNode true)
          (if (Variables|Default|GetIsOnLilyPad)
            (Variables|Default|SetIsOnLilyPad false)
            (Variables|/Game/Blueprints/BP_LilyPad.BP_LilyPad_C|SetHasChickenOnTop (Variables|Default|GetCurLilyPad) false))
          (CallFunction|CalcNewNodePos (Variables|Default|GetCurLandingNode))
          (if (Variables|/Game/Blueprints/BP_LandingNode.BP_LandingNode_C|GetIs%20Water (Variables|Default|GetCurLandingNode))
            (Variables|Default|SetFallIntoWaterAfterLand true)))
        (:CastFailed
          (bind _asbp_lily_pad (Utilities|Casting|CastToBP_LilyPad (.HitActor (Collision|BreakHitResult _array_element))))
          (Variables|Default|SetCurLilyPad _asbp_lily_pad)
          (Variables|Default|SetIsOnLog false)
          (Variables|Default|SetFoundLandingNode true)
          (Variables|Default|SetIsOnLilyPad true)
          (Variables|/Game/Blueprints/BP_Bounce.BP_Bounce_C|SetIsBeingJumpedOn (Variables|Default|GetCurLilyPad) true)
          (Variables|/Game/Blueprints/BP_LilyPad.BP_LilyPad_C|SetHasChickenOnTop (Variables|Default|GetCurLilyPad) true)))
      (CallFunction|PlayJumpingSounds)
      (goto _label Break))))

(fn PrepTraceforLandingNode
  (bind _returnvalue (Transformation|GetActorLocation))
  (bind _rayoriginrelative (Variables|Default|GetRayOriginRelative))
  (bind _returnvalue_2 (+ _rayoriginrelative _returnvalue))
  (CallFunction|TraceforLandingNode _returnvalue_2 (+ _returnvalue_2 "0, 0,-200.000000")))

(fn JumponLogAttempt
  (bind _returnvalue (Transformation|GetActorLocation))
  (bind _returnvalue_2 (Transformation|GetActorLocation))
  (bind _returnvalue_3 (Transformation|GetActorLocation))
  (bind _returnvalue_4 (Transformation|GetActorLocation))
  (bind _curlog (Variables|Default|GetCurLog))
  (bind _curdir (Variables|Default|GetCurDir))
  (bind _returnvalue_5 (== _curdir 0))
  (Utilities|IsValid _curlog
    (:Is%20Valid
      (if (Variables|/Game/Blueprints/BP_Log.BP_Log_C|GetMoveLeft _curlog)
        (if _returnvalue_5
          (Variables|Default|SetCurLandingNodePos (Math|Vector|MakeVector (- (.x _returnvalue) (LocalVariables|GetLogJumpXOffsetMagnitude)) (.y _returnvalue) (Variables|Default|GetOffsetDown)))
          (else
            (Variables|Default|SetCurLandingNodePos (Math|Vector|MakeVector (+ (.x _returnvalue_2) (LocalVariables|GetLogJumpXOffsetMagnitude)) (.y _returnvalue_2) (Variables|Default|GetOffsetDown)))))
        (elif _returnvalue_5
          (Variables|Default|SetCurLandingNodePos (Math|Vector|MakeVector (- (.x _returnvalue_4) (LocalVariables|GetLogJumpXOffsetMagnitude)) (.y _returnvalue_4) (Variables|Default|GetOffsetDown)))
          (else
            (Variables|Default|SetCurLandingNodePos (Math|Vector|MakeVector (+ (.x _returnvalue_3) (LocalVariables|GetLogJumpXOffsetMagnitude)) (.y _returnvalue_3) (Variables|Default|GetOffsetDown))))))
      (Variables|Default|SetFoundLogJumpHorizontalPos true)
      (Default|ResetAnim (Variables|Default|GetCurLog)))))

(fn JumpAnim
  (bind _output_get (LocalVariables|SetDistRatio (- (* (/ (Variables|Default|GetDistTraveled) (Variables|Default|GetDistToLandingNode)) 2.0) 1.0)))
  (Variables|Default|SetJumpingZAmount (* (+ (* (Math|Float|Square _output_get) -1.0) 1.0) 1e+02)))

(fn CalcNewLinearPos
  (Variables|Default|SetLinearXAmount (+ (Variables|Default|GetNodePosXDelta) (Variables|Default|GetLinearXAmount)))
  (Variables|Default|SetLinearYAmount (+ (Variables|Default|GetNodePosYDelta) (Variables|Default|GetLinearYAmount)))
  (Variables|Default|SetLinearZAmount (+ (Variables|Default|GetNodePosZDelta) (Variables|Default|GetLinearZAmount))))