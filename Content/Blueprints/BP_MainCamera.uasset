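; BP_MainCamera is the camera actor for a Crossy Road-style game, following the player's chicken along the Y axis.
; On BeginPlay it caches the player pawn as BP_Chicken and also passes that reference to the BP_CrossyRoad_GM game mode.
; Each Tick it moves itself to the chicken's Y plus an offset, keeping X and height fixed, with no smoothing.
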(event EventTick
  (params (DeltaSeconds :type Float%20%28single-precision%29))
  (Transformation|SetActorLocation (Math|Vector|MakeVector 0.0 (+ (.y (Transformation|GetActorLocation (Variables|Default|GetChickenREF))) (Variables|Default|GetOffsetY)) 1.3e+03) false false))

(event EventBeginPlay
  (bind _asbp_chicken (Utilities|Casting|CastToBP_Chicken (Game|Player|GetPlayerPawn 0)))
  (Variables|Default|SetChickenREF _asbp_chicken)
  (bind _asbp_crossy_road_gm (Utilities|Casting|CastToBP_CrossyRoad_GM (Game|GetGameMode)))
  (Variables|/Game/Blueprints/BP_CrossyRoad_GM.BP_CrossyRoad_GM_C|SetChickenREF _asbp_crossy_road_gm (Variables|Default|GetChickenREF)))

(fn ConstructionScript)