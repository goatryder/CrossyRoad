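; Game mode for a Crossy Road-style game that sets up input and camera, builds the terrain, and polls for game over to reload the Gameplay level.
; ConstructFloors spawns random grass, road, water and railroad chunks until rows reach 20 ahead of the player, with chunk length tied to progress.
; Shared clear-column positions carry between grass and water rows.
; Water rows limit same-direction log runs and allow lily pads only after logs in both directions.
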(event Custom|CheckIfGameOver
  ;[1 1 1] Check Game Over Every 1 Sec
  (if (Variables|Default|GetGameOver)
    (Variables|Default|SetIsGameOver false)
    (Utilities|FlowControl|Delay 3.0)
    (Game|OpenLevel(byName) "Gameplay")))

(event EventBeginPlay
  (bind _returnvalue (Game|GetPlayerController 0))
  (Utilities|FlowControl|Sequence
    (:then_0
      ;[1 1 1] Create UI
      (CallFunction|CreateUI))
    (:then_1
      ;[1 1 1] Enable Input And Show Cursor
      (Input|EnableInput _returnvalue 0)
      (Variables|/Script/Engine.PlayerController|SetbShowMouseCursor _returnvalue true))
    (:then_2
      ;[1 1 1] Set Camera
      (bind _outactors (Actor|GetAllActorswithTag "Camera"))
      (for _array_element _outactors
        (bind _asbp_main_camera (Utilities|Casting|CastToBP_MainCamera _array_element))
        (bind _output_get (Variables|Default|SetCameraREF _asbp_main_camera))
        (Game|Player|SetViewTargetwithBlend (Game|GetPlayerController 0) _output_get 0.0 "VTBlend_Linear" 0.0 false)))
    (:then_3
      ;[1 1 1] Construct Init Floors
      (CallFunction|ConstructInitFloors))
    (:then_4
      ;[1 1 1] Check Game Over Every 1 Sec
      (Utilities|Time|SetTimerbyEvent (delegate Custom|CheckIfGameOver) 1.0 true))))

(fn ConstructionScript)

(fn CalcNumLilyPadstoCreate
  (Variables|Default|SetNumLilyPadsToCreate 0)
  (Utilities|FlowControl|Sequence
    (:then_0
      (if (!= (Variables|Default|GetClearColumnPosX1) -1.0)
        (Math|Integer|IncrementInt (Variables|Default|GetNumLilyPadsToCreate))))
    (:then_1
      (if (!= (Variables|Default|GetClearColumnPosX2) -1.0)
        (Math|Integer|IncrementInt (Variables|Default|GetNumLilyPadsToCreate))))
    (:then_2
      (if (!= (Variables|Default|GetClearColumnPosX3) -1.0)
        (Math|Integer|IncrementInt (Variables|Default|GetNumLilyPadsToCreate))))))

(fn CreateClearColumnPos
  (Utilities|FlowControl|Sequence
    (:then_0
      (Variables|Default|SetClearColumnPosX1 -1.0))
    (:then_1
      (Variables|Default|SetClearColumnPosX2 -1.0))
    (:then_2
      (Variables|Default|SetClearColumnPosX3 -1.0)
      (for _index (range 0 (Math|Random|RandomInteger 3))
        (switch int _index
          (:0
            (Variables|Default|SetClearColumnPosX1 (- (* (Math|Random|RandomInteger 8) 2e+02) 8e+02)))
          (:1
            (Variables|Default|SetClearColumnPosX2 (- (* (Math|Random|RandomInteger 8) 2e+02) 8e+02)))
          (:2
            (Variables|Default|SetClearColumnPosX3 (- (* (Math|Random|RandomInteger 8) 2e+02) 8e+02))))))))

(fn CalcFloorSpawnY
  (return (- (* (Variables|Default|GetCurFloorIndex) (Variables|Default|GetFloorSpawnYDelta)) 2e+02)))

(fn CalcCurFoorTypetoCreate
  (Variables|Default|SetPrevFloorTypeCreated (Variables|Default|GetCurFloorTypeCreated))
  (Variables|Default|SetCurFloorTypeCreated (Math|Random|RandomInteger 4))
  (if (== (Variables|Default|GetCurFloorIndex) (Variables|Default|GetPrevFloorTypeCreated))
    (Variables|Default|SetCurFloorTypeCreated (Math|Integer|%(Integer) (+ (Variables|Default|GetPrevFloorTypeCreated) 1) 4))))

(fn CreateGrassFloorChunk
  (params (FloorNum :type Integer) (CenterClearColumn :type Boolean))
  (if (== (Variables|Default|GetPrevFloorTypeCreated) 2)
    _
    (else
      (CallFunction|CreateClearColumnPos)))
  (if CenterClearColumn
    (Variables|Default|SetClearColumnPosX3 0.0))
  (for _index (range 0 (- FloorNum 1))
    (Math|Integer|IncrementInt (Variables|Default|GetCurFloorIndex)
      (:%20%20
        (bind _positiony (CallFunction|CalcFloorSpawnY))
        (Game|SpawnActorfromClass "/Game/Blueprints/BP_Grass.BP_Grass_C" (Math|Transform|MakeTransform (Math|Vector|MakeVector 0.0 _positiony 0.0)) "Undefined" 0 (== (Math|Integer|%(Integer) _index 2) 1) (Variables|Default|GetClearColumnPosX1) (Variables|Default|GetClearColumnPosX2) (Variables|Default|GetClearColumnPosX3) (Variables|Default|GetChickenREF) _positiony 0)))))

(fn CreateRoadFloorChunk
  (params (FloorNum :type Integer))
  (for _index (range 0 (- FloorNum 1))
    (Math|Integer|IncrementInt (Variables|Default|GetCurFloorIndex)
      (:%20%20
        (bind _positiony (CallFunction|CalcFloorSpawnY))
        (Game|SpawnActorfromClass "/Game/Blueprints/BP_Road.BP_Road_C" (Math|Transform|MakeTransform (Math|Vector|MakeVector 0.0 _positiony 0.0)) "Undefined" 0 (or (>= (Math|Conversions|ToByte(Integer) _index) 1) (== (Variables|Default|GetPrevFloorTypeCreated) 1)) (Variables|Default|GetChickenREF) _positiony 0)))))

(fn CreateRailroadFloorChunk
  (params (FloorNum :type Integer))
  (for _index (range 0 (- FloorNum 1))
    (Math|Integer|IncrementInt (Variables|Default|GetCurFloorIndex)
      (:%20%20
        (bind _positiony (CallFunction|CalcFloorSpawnY))
        (Game|SpawnActorfromClass "/Game/Blueprints/BP_Railroad.BP_Railroad_C" (Math|Transform|MakeTransform (Math|Vector|MakeVector 0.0 _positiony 0.0)) "Undefined" 0 (Variables|Default|GetChickenREF) _positiony 0)))))

(fn CreateWaterFloorChunk
  (params (FloorNum :type Integer))
  (Variables|Default|SetCreatedLilyPadsSinceWaterChunkGroupStarted false)
  (for _index (range 0 (- FloorNum 1))
    (Math|Integer|IncrementInt (Variables|Default|GetCurFloorIndex)
      (:%20%20
        (bind _positiony (CallFunction|CalcFloorSpawnY))
        (LocalVariables|SetPosY _positiony)
        (if (== (Math|Random|RandomInteger 3) 0)
          (if (Variables|Default|GetCanCreateLilyPads)
            ;[1 1 1] Create Water Chunk With LilyPads
            (if (Variables|Default|GetCreatedLilyPadsSinceWaterChunkGroupStarted)
              (CallFunction|CreateClearColumnPos))
            (CallFunction|CalcNumLilyPadstoCreate)
            (Game|SpawnActorfromClass "/Game/Blueprints/BP_Water.BP_Water_C" (Math|Transform|MakeTransform (Math|Vector|MakeVector 0.0 (LocalVariables|GetPosY) 0.0) "0, 0, 0" "1,1,1") "Undefined" 0 false false true (Variables|Default|GetNumLilyPadsToCreate) (Variables|Default|GetClearColumnPosX1) (Variables|Default|GetClearColumnPosX2) (Variables|Default|GetClearColumnPosX3) (Variables|Default|GetChickenREF) (LocalVariables|GetPosY) 0)
            (Variables|Default|SetCreatedLilyPadsSinceWaterChunkGroupStarted true)
            (Variables|Default|SetCanCreateLilyPads false)
            (Variables|Default|SetCreatedLeftLogsSinceLilyPads false)
            (Variables|Default|SetCreatedRightLigsSinceLilyPads false)
            (else
              ;[1 1 1] Create Water Chunk With Logs
              (Utilities|FlowControl|Sequence :!label _label
                (:then_0
                  ;;[1 1 1] Calc Log Direction
                  (bind _output_get (Variables|Default|SetCreateLogsLeft (Math|Random|RandomBool)))
                  (if (Math|Boolean|Equal(Boolean) _output_get (Variables|Default|GetPreviousLogCreationDirection))
                    (bind _result (Math|Integer|IncrementInt (Variables|Default|GetNumLogsCreatedInSameDir))
                      (:%20%20
                        (if (> _result 2)
                          (bind _output_get_2 (Variables|Default|SetCreateLogsLeft (not (Variables|Default|GetCreateLogsLeft))))
                          (Variables|Default|SetNumLogsCreatedInSameDir 1)
                          (Variables|Default|SetPreviousLogCreationDirection _output_get_2))))
                    (else
                      (Variables|Default|SetNumLogsCreatedInSameDir 1))))
                (:then_1
                  (Game|SpawnActorfromClass "/Game/Blueprints/BP_Water.BP_Water_C" (Math|Transform|MakeTransform (Math|Vector|MakeVector 0.0 (LocalVariables|GetPosY) 0.0) "0, 0, 0" "1,1,1") "Undefined" 0 true (Variables|Default|GetCreateLogsLeft) false 0 (Variables|Default|GetClearColumnPosX1) (Variables|Default|GetClearColumnPosX2) (Variables|Default|GetClearColumnPosX3) (Variables|Default|GetChickenREF) (LocalVariables|GetPosY) 0)
                  (if (Variables|Default|GetCreateLogsLeft)
                    (Variables|Default|SetCreatedLeftLogsSinceLilyPads true)
                    (else
                      (Variables|Default|SetCreatedRightLigsSinceLilyPads true)))
                  (if (Variables|Default|GetCreatedLeftLogsSinceLilyPads)
                    (if (Variables|Default|GetCreatedRightLigsSinceLilyPads)
                      (Variables|Default|SetCanCreateLilyPads true)))
                  (Variables|Default|SetPreviousLogCreationDirection (Variables|Default|GetCreateLogsLeft))))))
          (else
            (goto _label)))))))

(fn CalcFloorNum
  (return (+ (Math|Random|RandomInteger (- 6 (/ (Variables|Default|GetNumChunksExploredFwd) 20))) 1)))

(fn ConstructFloors
  (bind _randfloornum (CallFunction|CalcFloorNum))
  (while (< (- (Variables|Default|GetCurFloorIndex) (Variables|Default|GetPlayerPosIndex)) 20)
    (CallFunction|CalcCurFoorTypetoCreate)
    (switch int (Variables|Default|GetCurFloorTypeCreated)
      (:0
        (if (< _randfloornum 1)
          (CallFunction|CreateGrassFloorChunk _randfloornum false)
          (else
            (CallFunction|CreateGrassFloorChunk 1 false))))
      (:1
        (CallFunction|CreateRoadFloorChunk (CallFunction|CalcFloorNum)))
      (:2
        (CallFunction|CreateWaterFloorChunk (CallFunction|CalcFloorNum)))
      (:3
        (CallFunction|CreateRailroadFloorChunk (CallFunction|CalcFloorNum))))))

(fn ConstructInitFloors
  (CallFunction|CreateGrassFloorChunk 8 false)
  (CallFunction|CreateGrassFloorChunk 2 true)
  (CallFunction|ConstructFloors))

(fn CreateUI)