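; BP_Road is a road floor chunk, apparently for a chicken road-crossing game, built on inherited floor-chunk logic.
; On BeginPlay it spawns left, center and right floors, with only the center traversable, plus optional lane-line props.
; It then adds a vehicle spawner on a random side, passing it the chicken reference, and builds landing nodes with coin attempts.
; Destroying the road also destroys its vehicle spawners.
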(event EventBeginPlay
  (|CallParentFunction)
  (CallFunction|CreateRoadFloors))

(event EventDestroyed
  (for _array_element (Variables|Default|GetVehicleSpawners)
    (Actor|DestroyActor _array_element)))

(fn ConstructionScript
  (|CallParentFunction))

(fn ConstructVehicleSpawner
  (params (Position%20Y :type Float%20%28single-precision%29))
  (bind _output_get (LocalVariables|SetFacingLeft (Math|Random|RandomBool)))
  (if _output_get
    (LocalVariables|SetPositionX 2.8e+03)
    (else
      (LocalVariables|SetPositionX -2.8e+03)))
  (bind _returnvalue (Game|SpawnActorfromClass "/Game/Blueprints/BP_VehicleSpawner.BP_VehicleSpawner_C" (Math|Transform|MakeTransform (Math|Vector|MakeVector (LocalVariables|GetPositionX) Position%20Y -1e+01)) "Undefined" 0 (LocalVariables|GetFacingLeft) (Variables|Default|GetChickenREF) 0))
  (Utilities|Array|Add (Variables|Default|GetVehicleSpawners) _returnvalue))

(fn ConstructLandingNodes
  (Variables|Default|SetCurrentZPosFromLandingNode -3e+01)
  (for _index (range 0 8)
    (CallFunction|AttemptingCoinCreation)
    (CallFunction|ConstructLandingNode(FloorChunk) false)))

(fn CreateRoadFloors
  (bind (_transformleft _transformmid _transofrmright _yposition) (CallFunction|CalcFloorTransform))
  (LocalVariables|SetYPosition _yposition)
  (bind _returnvalue (Game|SpawnActorfromClass "/Game/Blueprints/BP_Floor.BP_Floor_C" _transformleft "Undefined" 0 1 false self 0))
  (Variables|Default|SetLeftFloor _returnvalue)
  (bind _returnvalue_2 (Game|SpawnActorfromClass "/Game/Blueprints/BP_Floor.BP_Floor_C" _transformmid "Undefined" 0 1 true self 0))
  (Variables|Default|SetCenterFloor _returnvalue_2)
  (bind _returnvalue_3 (Game|SpawnActorfromClass "/Game/Blueprints/BP_Floor.BP_Floor_C" _transofrmright "Undefined" 0 1 false self 0))
  (Variables|Default|SetRightFloor _returnvalue_3)
  (Utilities|FlowControl|Sequence
    (:then_0
      (if (Variables|Default|GetHasLines)
        (bind _returnvalue_4 (Game|SpawnActorfromClass "/Game/Blueprints/BP_RoadLines.BP_RoadLines_C" (Math|Transform|MakeTransform (Math|Vector|MakeVector -2e+03 (+ (LocalVariables|GetYPosition) 1e+02) 0.0)) "Undefined" 0 true 0))
        (Utilities|Array|Add (Variables|Default|GetProps) _returnvalue_4)
        (bind _returnvalue_5 (Game|SpawnActorfromClass "/Game/Blueprints/BP_RoadLines.BP_RoadLines_C" (Math|Transform|MakeTransform (Math|Vector|MakeVector 0.0 (+ (LocalVariables|GetYPosition) 1e+02) 0.0)) "Undefined" 0 false 0))
        (Utilities|Array|Add (Variables|Default|GetProps) _returnvalue_5)
        (Game|SpawnActorfromClass "/Game/Blueprints/BP_RoadLines.BP_RoadLines_C" (Math|Transform|MakeTransform (Math|Vector|MakeVector 2e+03 (+ (LocalVariables|GetYPosition) 1e+02) 0.0)) "Undefined" 0 true 0)
        (Utilities|Array|Add (Variables|Default|GetProps) 0)))
    (:then_1
      (CallFunction|ConstructVehicleSpawner (LocalVariables|GetYPosition))
      (CallFunction|ConstructLandingNodes))))