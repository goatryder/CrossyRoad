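; BP_Railroad is a railroad floor chunk that trains periodically cross from a random side.
; On BeginPlay it spawns three floor sections with only the center traversable, adds track props, and builds landing nodes with coin creation attempts.
; Tick drives accumulated-time timers that spawn trains at random intervals, switch a warning light on and off, and trigger one of two train sounds.
; A warning sound plays as each new spawn countdown starts.
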(event EventBeginPlay
  (|CallParentFunction)
  (CallFunction|CreateRailroadFloors))

(event EventTick
  (params (DeltaSeconds :type Float%20%28single-precision%29))
  (CallFunction|ManageTrainSpawning DeltaSeconds)
  (CallFunction|ManageTrainLightVisibility DeltaSeconds)
  (CallFunction|ManagePlayTrainSound DeltaSeconds))

(fn ConstructionScript
  (|CallParentFunction))

(fn ConstructLandingNodes
  (Variables|Default|SetCurrentZPosFromLandingNode -3e+01)
  (for _index (range 0 8)
    (CallFunction|AttemptingCoinCreation)
    (CallFunction|ConstructLandingNode(FloorChunk) false)))

(fn CreateRailroadFloors
  (bind (_transformleft _transformmid _transofrmright _yposition) (CallFunction|CalcFloorTransform))
  (LocalVariables|SetYPosition _yposition)
  ;[1 1 1] Set Road Floors
  (bind _returnvalue (Game|SpawnActorfromClass "/Game/Blueprints/BP_Floor.BP_Floor_C" _transformleft "Undefined" 0 1 false self 0))
  (Variables|Default|SetLeftFloor _returnvalue)
  (bind _returnvalue_2 (Game|SpawnActorfromClass "/Game/Blueprints/BP_Floor.BP_Floor_C" _transformmid "Undefined" 0 1 true self 0))
  (Variables|Default|SetCenterFloor _returnvalue_2)
  (bind _returnvalue_3 (Game|SpawnActorfromClass "/Game/Blueprints/BP_Floor.BP_Floor_C" _transofrmright "Undefined" 0 1 false self 0))
  (Variables|Default|SetRightFloor _returnvalue_3)
  (Utilities|FlowControl|Sequence
    (:then_0
      ;[1 1 1] Add Rails Props To Road Floors
      (bind _returnvalue_4 (Game|SpawnActorfromClass "/Game/Blueprints/BP_Tracks.BP_Tracks_C" (Math|Transform|MakeTransform (Math|Vector|MakeVector -1.8e+03 (LocalVariables|GetYPosition) 0.0)) "Undefined" 0 true 0))
      (Utilities|Array|Add (Variables|Default|GetProps) _returnvalue_4)
      (bind _returnvalue_5 (Game|SpawnActorfromClass "/Game/Blueprints/BP_Tracks.BP_Tracks_C" (Math|Transform|MakeTransform (Math|Vector|MakeVector 0.0 (LocalVariables|GetYPosition) 0.0)) "Undefined" 0 false 0))
      (Utilities|Array|Add (Variables|Default|GetProps) _returnvalue_5)
      (Game|SpawnActorfromClass "/Game/Blueprints/BP_Tracks.BP_Tracks_C" (Math|Transform|MakeTransform (Math|Vector|MakeVector 1.8e+03 (LocalVariables|GetYPosition) 0.0)) "Undefined" 0 true 0)
      (Utilities|Array|Add (Variables|Default|GetProps) 0))
    (:then_1
      ;[1 1 1] Construct Landing Nodes
      (CallFunction|ConstructLandingNodes))))

(fn ManageTrainSpawning
  (params (DeltaSeconds :type Float%20%28single-precision%29))
  (if (Variables|Default|GetStartedSpawningTrainSession)
    (Variables|Default|SetMaxTrainSpawnTimeAccumulation (Math|Random|RandomFloatinRange 5.0 1e+01))
    (Variables|Default|SetStartedSpawningTrainSession false)
    (Variables|Default|SetCurTrainSpawnTimeAccomulation 0.0)
    ;[1 1 1] Play Train Warning Sound
    (Audio|Components|Audio|Play (Variables|Default|GetTrainWarningSound) 0.0)
    (else
      (bind _output_get (Variables|Default|SetCurTrainSpawnTimeAccomulation (+ DeltaSeconds (Variables|Default|GetCurTrainSpawnTimeAccomulation))))
      (if (>= _output_get (Variables|Default|GetMaxTrainSpawnTimeAccumulation))
        (Variables|Default|SetStartedSpawningTrainSession true)
        ;[1 1 1] Spawn Train
        (LocalVariables|SetMoveLeft (Math|Random|RandomBool))
        (|SetTrainSpawnLocation)
        (Game|SpawnActorfromClass "/Game/Blueprints/BP_Train.BP_Train_C" (Math|Transform|MakeTransform (LocalVariables|GetSpawnLocation) "0, 0, 0" "1,1,1") "Undefined" 0 (LocalVariables|GetMoveLeft) 0)
        ;[1 1 1] Enable Light
        (Rendering|SetVisibility (Variables|Default|GetPointLight) true false)
        (Variables|Default|SetTrainLightEnabled true)
        (Variables|Default|SetStartedPlayingTrainSound true)))))

(fn ManageTrainLightVisibility
  (params (DeltaSeconds :type Float%20%28single-precision%29))
  (if (Variables|Default|GetTrainLightEnabled)
    (bind _output_get (Variables|Default|SetCurLightTimeAccomulation (+ DeltaSeconds (Variables|Default|GetCurLightTimeAccomulation))))
    (if (>= _output_get (Variables|Default|GetMaxLightTimeAccomulation))
      (Variables|Default|SetCurLightTimeAccomulation 0.0)
      (Rendering|SetVisibility (Variables|Default|GetPointLight) false false)
      (Variables|Default|SetTrainLightEnabled false))))

(fn ManagePlayTrainSound
  (params (DeltaSeconds :type Float%20%28single-precision%29))
  (if (Variables|Default|GetStartedPlayingTrainSound)
    (bind _output_get (Variables|Default|SetCurTrainSoundAccomulation (+ DeltaSeconds (Variables|Default|GetCurTrainSpawnTimeAccomulation))))
    (if (>= _output_get (Variables|Default|GetMaxTrainSoundAccomulation))
      (|PlaySound)
      (Variables|Default|SetStartedPlayingTrainSound false)
      (Variables|Default|SetCurTrainSoundAccomulation 0.0))))