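; BP_Floor is a floor tile actor that displays as grass, road or water and visually marks whether it is traversable.
; On BeginPlay, a MultiGate uses FloorType as its start index, acting as a switch that passes the matching mesh to SetMesh.
; SetMesh applies the mesh with a new dynamic material instance, then calls DarkenMesh to lower the "darkness" parameter when the tile is not traversable.
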(event EventBeginPlay
  (Utilities|FlowControl|MultiGate false false (Variables|Default|GetFloorType)
    (:Out%200
      (CallFunction|SetMesh "/Game/media/meshes/grass.grass"))
    (:Out%201
      (CallFunction|SetMesh "/Game/media/meshes/road.road"))
    (:Out%202
      (CallFunction|SetMesh "/Game/media/meshes/water.water"))))

(fn ConstructionScript)

(fn DarkenMesh
  (params (Material%20Instance :type Material%20Instance%20Dynamic%20Object%20Reference))
  (bind _returnvalue (Rendering|Material|GetVectorParameterValue Material%20Instance "darkness" :!class /Script/Engine.MaterialInstanceDynamic))
  (Rendering|Material|SetVectorParameterValue Material%20Instance "darkness" (Math|Conversions|ToLinearColor(Float) (- (.R (Utilities|Struct|BreakLinearColor _returnvalue)) 0.4)) :!class /Script/Engine.MaterialInstanceDynamic))

(fn SetMesh
  (params (StaticMesh :type Static%20Mesh%20Object%20Reference))
  (Components|StaticMesh|SetStaticMesh (Variables|Default|GetFloorMesh) StaticMesh)
  (bind _returnvalue (Rendering|Material|CreateDynamicMaterialInstance (Variables|Default|GetFloorMesh) 0 "/Game/media/meshes/M_chicken__colors_png.M_chicken__colors_png" "None" :!class /Script/Engine.PrimitiveComponent))
  (bind _output_get (Variables|Default|SetMaterialInstance _returnvalue))
  (if (not (Variables|Default|GetTraversable))
    (CallFunction|DarkenMesh _output_get)))