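; Spawns a one-directional stream of BP_Vehicle actors along the X axis, passing each a facing, a chicken reference and a random speed shared per spawner.
; Tick accumulates time and spawns at the spawner's transform, re-rolling a 2–5 second interval each time.
; BeginPlay also runs a pre-fill loop that spawns at a fixed, facing-dependent X offset.
; The loop's random accumulators never feed the spawn location, and it never updates its ContinueCreatingVehicles condition.
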(event EventBeginPlay
  (Variables|Default|SetSpeed (Math|Random|RandomFloatinRange 3e+02 6e+02))
  (CallFunction|SetNewMaxTimeforSpawn)
  (CallFunction|SpawnInitialVehicles))

(event EventTick
  (params (DeltaSeconds :type Float%20%28single-precision%29))
  (bind _output_get (Variables|Default|SetTimeAccumulation (+ DeltaSeconds (Variables|Default|GetTimeAccumulation))))
  (if (>= _output_get (Variables|Default|GetTimeMaxForSpawn))
    (Variables|Default|SetTimeAccumulation 0.0)
    (CallFunction|SetNewMaxTimeforSpawn)
    (Game|SpawnActorfromClass "/Game/Blueprints/BP_Vehicle.BP_Vehicle_C" (Transformation|GetActorTransform) "Undefined" 0 (Variables|Default|GetFacingLeft) (Variables|Default|GetSpeed) (Variables|Default|GetChickenREF) 0)))

(fn ConstructionScript)

(fn SetNewMaxTimeforSpawn
  (Variables|Default|SetTimeMaxForSpawn (Math|Random|RandomFloatinRange 2.0 5.0)))

(fn SpawnInitialVehicles
  (bind _returnvalue (Transformation|GetActorLocation))
  (bind _returnvalue_2 (Math|Random|RandomFloatinRange 6e+02 1.2e+03))
  (bind _returnvalue_3 (Transformation|GetActorLocation))
  (if (Variables|Default|GetFacingLeft)
    (LocalVariables|SetXOffsetInit (+ (.x _returnvalue) -6e+02))
    (else
      (LocalVariables|SetXOffsetInit (+ (.x _returnvalue) 6e+02))))
  (while (LocalVariables|GetContinueCreatingVehicles)
    (LocalVariables|SetXOffsetAccomulation _returnvalue_2)
    (LocalVariables|SetDistanceAccomulation (+ _returnvalue_2 (LocalVariables|GetDistanceAccomulation)))
    (if (Variables|Default|GetFacingLeft)
      (LocalVariables|SetXOffsetAccomulation (* (LocalVariables|GetXOffsetAccomulation) -1.0)))
    (Game|SpawnActorfromClass "/Game/Blueprints/BP_Vehicle.BP_Vehicle_C" (Math|Transform|MakeTransform (Math|Vector|MakeVector (LocalVariables|GetXOffsetInit) (.y _returnvalue_3) (.z _returnvalue_3))) "Undefined" 0 (Variables|Default|GetFacingLeft) (Variables|Default|GetSpeed) (Variables|Default|GetChickenREF) 0)))