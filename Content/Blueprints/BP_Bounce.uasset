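; BP_Bounce is an actor that plays a short procedural vertical bounce when it is jumped on.
; While IsBeingJumpedOn is true, Tick accumulates time and, after a start delay, computes a parabolic Z offset applied to CachedZPos.
; The animation resets 0.2 seconds after that delay, returning the actor to its cached height.
; The flag and cached height are not set up in these graphs.
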(event EventBeginPlay
  (Variables|Default|SetMaxJumpOnTime (+ (Variables|Default|GetMaxStartJumpTime) 0.2)))

(event EventTick
  (params (DeltaSeconds :type Float%20%28single-precision%29))
  (CallFunction|BouncingAnim DeltaSeconds))

(fn ConstructionScript)

(fn ResetAnim
  (Variables|Default|SetIsBeingJumpedOn false)
  (Variables|Default|SetJumpedOnZOffset 0.0)
  (Variables|Default|SetCurrentJumpedOnTime 0.0))

(fn JumpedonAnim
  (params (DeltaTime :type Float%20%28single-precision%29))
  (Variables|Default|SetCurrentJumpedOnTime (+ DeltaTime (Variables|Default|GetCurrentJumpedOnTime)))
  (if (>= (Variables|Default|GetCurrentJumpedOnTime) (Variables|Default|GetMaxStartJumpTime))
    (if (>= (Variables|Default|GetCurrentJumpedOnTime) (Variables|Default|GetMaxJumpOnTime))
      (CallFunction|ResetAnim)
      (else
        (Variables|Default|SetJumpedOnZOffset (* (- (Math|Float|Square (- (* (- (Variables|Default|GetCurrentJumpedOnTime) 0.1) 8.0) 1.0)) 1.0) 2e+01))))))

(fn BouncingAnim
  (params (DeltaTime :type Float%20%28single-precision%29))
  (bind _returnvalue (Transformation|GetActorLocation))
  (if (Variables|Default|GetIsBeingJumpedOn)
    (CallFunction|JumpedonAnim DeltaTime)
    (Transformation|SetActorLocation (Math|Vector|MakeVector (.x _returnvalue) (.y _returnvalue) (+ (Variables|Default|GetCachedZPos) (Variables|Default|GetJumpedOnZOffset))) false false)))