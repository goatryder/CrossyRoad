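; Lily pad actor that bounces and reacts to a chicken landing on it, with parent BeginPlay logic preserved.
; BeginPlay picks a random yaw spin rate and has a one-in-three chance to spawn an actor at the pad's location.
; Tick plays a 2D sound as a jump-on starts, runs the bounce animation and spins the pad while a chicken is on top.
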(event EventBeginPlay
  (|CallParentFunction)
  (Variables|Default|SetRotation (Math|Rotator|MakeRotator 0.0 0.0 (Math|Random|RandomFloatinRange -2e+01 2e+01)))
  (switch int (Math|Random|RandomInteger 3)
    (:0
      (Game|SpawnActorfromClass "/Game/Blueprints/BP_Coin.BP_Coin_C" (Math|Transform|MakeTransform (Transformation|GetActorLocation) "0, 0, 0" "1,1,1") "Undefined" 0 0))))

(event EventTick
  (params (DeltaSeconds :type Float%20%28single-precision%29))
  (CallFunction|AttempPlayJumpedonSound)
  (CallFunction|BouncingAnim DeltaSeconds)
  (if (Variables|Default|GetHasChickenOnTop)
    (Transformation|AddActorLocalRotation (* (Variables|Default|GetRotation) DeltaSeconds) false false)))

(fn ConstructionScript
  (|CallParentFunction))

(fn AttempPlayJumpedonSound
  (if (and (== (Variables|Default|GetCurrentJumpedOnTime) 0.0) (Variables|Default|GetIsBeingJumpedOn))
    (Audio|PlaySound2D "/Game/media/sounds/lily_pad.lily_pad" 1.0 1.0 0.0 0 0)))